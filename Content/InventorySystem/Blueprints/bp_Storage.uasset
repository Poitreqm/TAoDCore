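; Item storage container that holds a slot array seeded from start items and exchanges items with the player's inventory.
; Slot functions add, stack, split overflow recursively, swap and remove items, refreshing the matching slot in the Storage widget from the player's main UI.
; Dropped items spawn as pickup actors at a clear spot found by rotating the player's capsule and line tracing forward, falling back to the capsule location.
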(event `self.ReceiveBeginPlay`
  (set `self.Slots` (`self.StartItems`))
  (set `self.StorageWidget` (`/Game/InventorySystem/Widgets/w_MainWidget.Storage` (`/Game/InventorySystem/Blueprints/bp_Inventory.MainWidget` (`/Game/Core/Blueprints/TopDownCharacter.InventoryRef` (`self.TopDownCharRef`)))))
  (`KismetArrayLibrary.Array_Resize` (`self.Slots`) (`self.AmountOfSlots`)))

(event `UpdateSlotAtIndex`
  (params (Index :type Integer))
  (`/Game/InventorySystem/Widgets/Storage/w_StorageSlot.UpdateSlot` (`|GetArrayItem` (`/Game/InventorySystem/Widgets/Storage/w_StorageWidget.SlotsWidgets` (`self.StorageWidget`)) Index)))

(fn `-AddItem`
  (params (ItemClass :type "/Game/InventorySystem/Blueprints/ItemClasses/Classes/bp_MasterItem Class Reference") (Amount :type Integer))
  (returns (`Success?` :type Boolean) (Rest :type Integer))
  (locals (local_FoundIndex :type Integer :default 0) (local_ItemClass :type "/Game/InventorySystem/Blueprints/ItemClasses/Classes/bp_MasterItem Class Reference") (local_Amount :type Integer))
  (bind _slots (`self.Slots`))
  (bind _local_foundindex (`local.local_FoundIndex`))
  (bind _local_itemclass (`local.local_ItemClass`))
  (bind _local_amount (`local.local_Amount`))
  (bind _returnvalue (+ (`.Amount_5_A24D12CF4AB976D01465479176E6C97A` (break `/Game/InventorySystem/Blueprints/Structures/s_InventorySlot` (`|GetArrayItem` (`self.Slots`) (`local.local_FoundIndex`)))) (`local.local_Amount`)))
  (set `local.local_ItemClass` ItemClass)
  (set `local.local_Amount` Amount)
  (if (`.canBeStacked?_16_6B51DF5D483FF839CD851BBD1EEFA1DA` (break `/Game/InventorySystem/Blueprints/Structures/s_ItemInfo` (defaults `Object` ItemClass)))
    (bind (_success_ _index) (`self.-SearchFreeStack` (`local.local_ItemClass`)))
    (if _success_
      (set `local.local_FoundIndex` _index)
      (if (> _returnvalue (`self.MaxStackSize`))
        (set `local.local_Amount` (- _returnvalue (`self.MaxStackSize`)))
        (`KismetArrayLibrary.Array_Set` _slots _local_foundindex (make `/Game/InventorySystem/Blueprints/Structures/s_InventorySlot` _local_itemclass (`self.MaxStackSize`)))
        (`self.UpdateSlotAtIndex` (`local.local_FoundIndex`))
        (bind (_success__2 _rest) (`self.-AddItem` (`local.local_ItemClass`) (`local.local_Amount`)))
        (return _success__2 _rest)
        (else
          (`KismetArrayLibrary.Array_Set` _slots _local_foundindex (make `/Game/InventorySystem/Blueprints/Structures/s_InventorySlot` _local_itemclass _returnvalue))
          (`self.UpdateSlotAtIndex` (`local.local_FoundIndex`))
          (return true 0)))
      (else
        (bind (_success__3 _index_2) (`self.-SearchEmptySlot`))
        (if _success__3
          (bind _output_get (set `local.local_FoundIndex` _index_2))
          (if (> (`local.local_Amount`) (`self.MaxStackSize`))
            (`KismetArrayLibrary.Array_Set` (`self.Slots`) _output_get (make `/Game/InventorySystem/Blueprints/Structures/s_InventorySlot` (`local.local_ItemClass`) (`self.MaxStackSize`)))
            (`self.UpdateSlotAtIndex` (`local.local_FoundIndex`))
            (bind (_success__4 _rest_2) (`self.-AddItem` (`local.local_ItemClass`) (- (`local.local_Amount`) (`self.MaxStackSize`))))
            (return _success__4 _rest_2)
            (else
              (`KismetArrayLibrary.Array_Set` (`self.Slots`) (`local.local_FoundIndex`) (make `/Game/InventorySystem/Blueprints/Structures/s_InventorySlot` (`local.local_ItemClass`) (`local.local_Amount`)))
              (`self.UpdateSlotAtIndex` (`local.local_FoundIndex`))
              (return true 0)))
          (else
            (return false (`local.local_Amount`))))))
    (else
      (bind (_success__5 _index_3) (`self.-SearchEmptySlot`))
      (if _success__5
        (bind _output_get_2 (set `local.local_FoundIndex` _index_3))
        (`KismetArrayLibrary.Array_Set` (`self.Slots`) _output_get_2 (make `/Game/InventorySystem/Blueprints/Structures/s_InventorySlot` (`local.local_ItemClass`) 1))
        (`self.UpdateSlotAtIndex` (`local.local_FoundIndex`))
        (if (> _local_amount 1)
          (bind (_success__6 _rest_3) (`self.-AddItem` (`local.local_ItemClass`) (- _local_amount 1)))
          (return true _rest_3)
          (else
            (return true 0)))
        (else
          (return false (`local.local_Amount`)))))))

(fn `-AddItemToIndex`
  (params (Index :type Integer) (Amount :type Integer) (ItemClass :type "/Game/InventorySystem/Blueprints/ItemClasses/Classes/bp_MasterItem Class Reference"))
  (returns (`Success?` :type Boolean))
  (if (and (`self.-IsSlotEmpty?` Index) (<= Amount (`self.MaxStackSize`)))
    (`KismetArrayLibrary.Array_Set` (`self.Slots`) Index (make `/Game/InventorySystem/Blueprints/Structures/s_InventorySlot` ItemClass Amount))
    (`self.UpdateSlotAtIndex` Index)
    (return true)
    (else
      (return false))))

(fn `-AddToIndex`
  (params (FromIndex :type Integer) (ToIndex :type Integer))
  (returns (`Success?` :type Boolean))
  (locals (local_From :type Integer) (local_To :type Integer) (local_Class :type "/Game/InventorySystem/Blueprints/ItemClasses/Classes/bp_MasterItem Class Reference"))
  (bind (_output_itemclass _output_amount) (break `/Game/InventorySystem/Blueprints/Structures/s_InventorySlot` (`|GetArrayItem` (`self.Slots`) (`local.local_To`))))
  (bind _output_itemclass_2 (break `/Game/InventorySystem/Blueprints/Structures/s_InventorySlot` (`|GetArrayItem` (`self.Slots`) (`local.local_From`))))
  (set `local.local_From` FromIndex)
  (set `local.local_To` ToIndex)
  (if (and (== _output_itemclass_2 _output_itemclass) (< _output_amount (`self.MaxStackSize`)) (`.canBeStacked?_16_6B51DF5D483FF839CD851BBD1EEFA1DA` (break `/Game/InventorySystem/Blueprints/Structures/s_ItemInfo` (`.Item Info` (`self.-GetItemInfoAtIndex` (`local.local_From`))))))
    (set `local.local_Class` _output_itemclass_2)
    (if (>= (- (`self.MaxStackSize`) (`self.-GetAmountAtIndex` (`local.local_To`))) (`self.-GetAmountAtIndex` (`local.local_From`)))
      (`KismetArrayLibrary.Array_Set` (`self.Slots`) (`local.local_To`) (make `/Game/InventorySystem/Blueprints/Structures/s_InventorySlot` (`local.local_Class`) (+ (`self.-GetAmountAtIndex` (`local.local_From`)) (`self.-GetAmountAtIndex` (`local.local_To`)))))
      (`KismetArrayLibrary.Array_Set` (`self.Slots`) (`local.local_From`) (make `/Game/InventorySystem/Blueprints/Structures/s_InventorySlot` null))
      (else
        (`KismetArrayLibrary.Array_Set` (`self.Slots`) (`local.local_From`) (make `/Game/InventorySystem/Blueprints/Structures/s_InventorySlot` (`local.local_Class`) (- (`self.-GetAmountAtIndex` (`local.local_From`)) (- (`self.MaxStackSize`) (`self.-GetAmountAtIndex` (`local.local_To`))))))
        (`KismetArrayLibrary.Array_Set` (`self.Slots`) (`local.local_To`) (make `/Game/InventorySystem/Blueprints/Structures/s_InventorySlot` (`local.local_Class`) (`self.MaxStackSize`)))))
    (`self.UpdateSlotAtIndex` (`local.local_From`))
    (`self.UpdateSlotAtIndex` (`local.local_To`))
    (return true)
    (else
      (return false))))

(fn `-GetAmountAtIndex`
  (params (Index :type Integer))
  (returns (Amount :type Integer))
  (return (`.Amount_5_A24D12CF4AB976D01465479176E6C97A` (break `/Game/InventorySystem/Blueprints/Structures/s_InventorySlot` (`|GetArrayItem` (`self.Slots`) Index)))))

(fn `-GetItemInfoAtIndex`
  (params (Index :type Integer))
  (returns (`Empty Slot?` :type Boolean) (`Item Info` :type "/Game/InventorySystem/Blueprints/Structures/s_ItemInfo Structure") (Amount :type Integer))
  (bind (_itemclass _amount) (break `/Game/InventorySystem/Blueprints/Structures/s_InventorySlot` (`|GetArrayItem` (`self.Slots`) Index)))
  (if (`KismetSystemLibrary.IsValidClass` _itemclass)
    (return false (defaults `Object` _itemclass) _amount)
    (else
      (return true (struct) 0))))

(fn `-IncreaseAmountAtIndex`
  (params (Index :type Integer) (Amount :type Integer))
  (returns (`Success?` :type Boolean))
  (bind _slots (`self.Slots`))
  (bind (_output_itemclass _output_amount) (break `/Game/InventorySystem/Blueprints/Structures/s_InventorySlot` (`|GetArrayItem` _slots Index)))
  (if (and (not (`self.-IsSlotEmpty?` Index)) (<= (+ (`self.-GetAmountAtIndex` Index) Amount) (`self.MaxStackSize`)))
    (`KismetArrayLibrary.Array_Set` _slots Index (make `/Game/InventorySystem/Blueprints/Structures/s_InventorySlot` _output_itemclass (+ _output_amount Amount)))
    (`self.UpdateSlotAtIndex` Index)
    (return true)
    (else
      (return false))))

(fn `-IsSlotEmpty?`
  (params (Index :type Integer))
  (returns (Empty :type Boolean))
  (return (not (`KismetSystemLibrary.IsValidClass` (`.ItemClass_3_6E81B15240E18385B7F49EAFAFC4F40B` (break `/Game/InventorySystem/Blueprints/Structures/s_InventorySlot` (`|GetArrayItem` (`self.Slots`) Index)))))))

(fn `-MovAllToInventory`
  (params (Inventory :type "/Game/InventorySystem/Blueprints/bp_Inventory Object Reference"))
  (locals (local_inv :type "/Game/InventorySystem/Blueprints/bp_Inventory Object Reference"))
  (bind _output_get (set `local.local_inv` Inventory))
  (`/Engine/EditorBlueprintResources/StandardMacros.IsValid` _output_get
    (:`Is Valid`
      (for (_array_element _array_index) (`self.Slots`)
        (bind (_itemclass _amount) (break `/Game/InventorySystem/Blueprints/Structures/s_InventorySlot` _array_element))
        (if (`KismetSystemLibrary.IsValidClass` _itemclass)
          (bind (_success2_ _rest2) (`/Game/InventorySystem/Blueprints/bp_Inventory.-AddItem` (`local.local_inv`) _itemclass _amount false 0))
          (if _success2_
            (`self.-RemoveItemAtIndex` _array_index (- _amount _rest2)))))
      (return))
    (:`Is Not Valid`
      (return))))

(fn `-MoveFromInvToStorageIndex`
  (params (Inventory :type "/Game/InventorySystem/Blueprints/bp_Inventory Object Reference") (InventoryIndex :type Integer) (StorageIndex :type Integer))
  (returns (`Success?` :type Boolean))
  (locals (local_Inventory :type "/Game/InventorySystem/Blueprints/bp_Inventory Object Reference") (local_InvIndex :type Integer) (local_StorageIndex :type Integer) (local_AmountToAdd :type Integer :default 0))
  (bind _local_inventory (`local.local_Inventory`))
  (bind _amount (`/Game/InventorySystem/Blueprints/bp_Inventory.-GetAmountAtIndex` (`local.local_Inventory`) (`local.local_InvIndex`)))
  (bind _returnvalue (- (`self.MaxStackSize`) (`self.-GetAmountAtIndex` (`local.local_StorageIndex`))))
  (set `local.local_Inventory` Inventory)
  (set `local.local_InvIndex` InventoryIndex)
  (bind _output_get (set `local.local_StorageIndex` StorageIndex))
  (if (`self.-IsSlotEmpty?` _output_get)
    (set `local.local_AmountToAdd` (`/Game/InventorySystem/Blueprints/bp_Inventory.-GetAmountAtIndex` _local_inventory (`local.local_InvIndex`)))
    (bind _success_ (`self.-AddItemToIndex` (`local.local_StorageIndex`) (`local.local_AmountToAdd`) (`.ItemClass_3_6E81B15240E18385B7F49EAFAFC4F40B` (break `/Game/InventorySystem/Blueprints/Structures/s_InventorySlot` (`|GetArrayItem` (`/Game/InventorySystem/Blueprints/bp_Inventory.Slots` _local_inventory) (`local.local_InvIndex`))))))
    (if _success_
      (`/Game/InventorySystem/Blueprints/bp_Inventory.-RemoveItemAtIndex` (`local.local_Inventory`) (`local.local_InvIndex`) (`local.local_AmountToAdd`) false)
      (return true)
      (else
        (return false)))
    (elif (and (== (`.ItemClass_3_6E81B15240E18385B7F49EAFAFC4F40B` (break `/Game/InventorySystem/Blueprints/Structures/s_InventorySlot` (`|GetArrayItem` (`self.Slots`) (`local.local_StorageIndex`)))) (`.ItemClass_3_6E81B15240E18385B7F49EAFAFC4F40B` (break `/Game/InventorySystem/Blueprints/Structures/s_InventorySlot` (`|GetArrayItem` (`/Game/InventorySystem/Blueprints/bp_Inventory.Slots` (`local.local_Inventory`)) (`local.local_InvIndex`))))) (`.canBeStacked?_16_6B51DF5D483FF839CD851BBD1EEFA1DA` (break `/Game/InventorySystem/Blueprints/Structures/s_ItemInfo` (`.Item Info` (`self.-GetItemInfoAtIndex` (`local.local_StorageIndex`))))) (< (`self.-GetAmountAtIndex` (`local.local_StorageIndex`)) (`self.MaxStackSize`)))
      (set `local.local_AmountToAdd` (select `bool` (> _amount _returnvalue) :`false` _amount :`true` _returnvalue))
      (bind _success__2 (`self.-IncreaseAmountAtIndex` (`local.local_StorageIndex`) (`local.local_AmountToAdd`)))
      (if _success__2
        (`/Game/InventorySystem/Blueprints/bp_Inventory.-RemoveItemAtIndex` (`local.local_Inventory`) (`local.local_InvIndex`) (`local.local_AmountToAdd`) false)
        (return true)
        (else
          (return false)))
      (else
        (return false)))))

(fn `-RemoveItemAtIndex`
  (params (Index :type Integer) (Amount :type Integer) (`isSpawn?` :type Boolean))
  (returns (`Success?` :type Boolean))
  (locals (local_Index :type Integer) (local_Amount :type Integer) (local_SpawnItem :type "/Game/InventorySystem/Blueprints/Structures/s_InventorySlot Structure"))
  (bind _slots (`self.Slots`))
  (bind _local_index (`local.local_Index`))
  (bind (_output_itemclass _output_amount) (break `/Game/InventorySystem/Blueprints/Structures/s_InventorySlot` (`|GetArrayItem` _slots _local_index)))
  (set `local.local_Index` Index)
  (set `local.local_Amount` Amount)
  (if (and (not (`self.-IsSlotEmpty?` (`local.local_Index`))) (> (`local.local_Amount`) 0))
    (set `local.local_SpawnItem` (`|GetArrayItem` (`self.Slots`) (`local.local_Index`)))
    (if (>= (`local.local_Amount`) (`self.-GetAmountAtIndex` (`local.local_Index`)))
      (`KismetArrayLibrary.Array_Set` (`self.Slots`) (`local.local_Index`) (make `/Game/InventorySystem/Blueprints/Structures/s_InventorySlot` null))
      (`self.UpdateSlotAtIndex` (`local.local_Index`))
      (else
        (`KismetArrayLibrary.Array_Set` _slots _local_index (make `/Game/InventorySystem/Blueprints/Structures/s_InventorySlot` _output_itemclass (- _output_amount (`local.local_Amount`))))
        (`self.UpdateSlotAtIndex` (`local.local_Index`))))
    (if `isSpawn?`
      (`self.-SpawnItemsClassInWorld` (`.ItemClass_3_6E81B15240E18385B7F49EAFAFC4F40B` (break `/Game/InventorySystem/Blueprints/Structures/s_InventorySlot` (`local.local_SpawnItem`))) (`local.local_Amount`))
      (return true)
      (else
        (return true)))
    (else
      (return false))))

(fn `-SearchEmptySlot`
  (returns (`Success?` :type Boolean) (Index :type Integer))
  (locals (local_Bool :type Boolean) (LocalIndex :type Integer))
  (for (_array_element _array_index) (`self.Slots`)
    (if (not (`KismetSystemLibrary.IsValidClass` (`.ItemClass_3_6E81B15240E18385B7F49EAFAFC4F40B` (break `/Game/InventorySystem/Blueprints/Structures/s_InventorySlot` _array_element))))
      (set `local.local_Bool` true)
      (set `local.LocalIndex` _array_index)
      (break)))
  (return (`local.local_Bool`) (`local.LocalIndex`)))

(fn `-SearchFreeStack`
  (params (ItemClass :type "/Game/InventorySystem/Blueprints/ItemClasses/Classes/bp_MasterItem Class Reference"))
  (returns (`Success?` :type Boolean) (Index :type Integer))
  (locals (local_Bool :type Boolean) (local_Index :type Integer))
  (for (_array_element _array_index) (`self.Slots`)
    (bind (_itemclass _amount) (break `/Game/InventorySystem/Blueprints/Structures/s_InventorySlot` _array_element))
    (if (`KismetSystemLibrary.IsValidClass` _itemclass)
      (if (and (== _itemclass ItemClass) (< _amount (`self.MaxStackSize`)))
        (set `local.local_Bool` true)
        (set `local.local_Index` _array_index)
        (break))))
  (return (`local.local_Bool`) (`local.local_Index`)))

(fn `-ShowHideStorage`
  (params (`Show?` :type Boolean))
  (if `Show?`
    (`Widget.SetVisibility` (`self.StorageWidget`) "Visible")
    (set `/Game/InventorySystem/Blueprints/bp_Inventory.StorageOpen?` true (`/Game/Core/Blueprints/TopDownCharacter.InventoryRef` (`self.TopDownCharRef`)))
    (else
      (`Widget.SetVisibility` (`self.StorageWidget`) "Hidden")
      (set `/Game/InventorySystem/Blueprints/bp_Inventory.StorageOpen?` false (`/Game/Core/Blueprints/TopDownCharacter.InventoryRef` (`self.TopDownCharRef`)))))
  (return))

(fn `-SpawnItemsClassInWorld`
  (params (ItemClass :type "/Game/InventorySystem/Blueprints/ItemClasses/Classes/bp_MasterItem Class Reference") (Amount :type Integer))
  (locals (local_Rotation :type Integer) (local_ItemClass :type "/Game/InventorySystem/Blueprints/ItemClasses/Classes/bp_MasterItem Class Reference") (local_Amount :type Integer) (local_ThrowAway :type Boolean))
  (bind _capsulecomponent (`Character.CapsuleComponent` (`self.TopDownCharRef`)))
  (bind _capsulecomponent_2 (`Character.CapsuleComponent` (`self.TopDownCharRef`)))
  (bind _returnvalue (`SceneComponent.K2_GetComponentLocation` _capsulecomponent))
  (set `local.local_ItemClass` ItemClass)
  (set `local.local_Amount` Amount)
  (for _ (range 361)
    (bind _output_get (set `local.local_Rotation` (+ (`local.local_Rotation`) 20)))
    (`SceneComponent.K2_SetWorldRotation` _capsulecomponent (`KismetMathLibrary.MakeRotator` (.roll (`SceneComponent.K2_GetComponentRotation` _capsulecomponent)) (.pitch (`SceneComponent.K2_GetComponentRotation` _capsulecomponent)) (+ (.yaw (`SceneComponent.K2_GetComponentRotation` _capsulecomponent)) (`KismetMathLibrary.Conv_IntToDouble` _output_get))) false false)
    (bind (_outhit _returnvalue_2) (`KismetSystemLibrary.LineTraceSingle` :`Start` _returnvalue :`End` (+ _returnvalue (* (`SceneComponent.GetForwardVector` _capsulecomponent) (`self.DistanceSpawnItem`))) :`TraceChannel` "TraceTypeQuery1" :`DrawDebugType` "ForDuration"))
    (if (not _returnvalue_2)
      (`|SpawnActorFromClass` "/Game/InventorySystem/Blueprints/ItemClasses/bp_PickupActor.bp_PickupActor_C" (`KismetMathLibrary.MakeTransform` (+ (* (`SceneComponent.GetForwardVector` _capsulecomponent_2) (`self.DistanceSpawnItem`)) (`SceneComponent.K2_GetComponentLocation` _capsulecomponent_2)) (.rotation (`.WorldView_36_43EFD57C4C969519E567A989749D17E2` (break `/Game/InventorySystem/Blueprints/Structures/s_ItemInfo` (defaults `Object` (`local.local_ItemClass`))))) (.scale (`.WorldView_36_43EFD57C4C969519E567A989749D17E2` (break `/Game/InventorySystem/Blueprints/Structures/s_ItemInfo` (defaults `Object` (`local.local_ItemClass`)))))) "Undefined" "OverrideRootScale" null (`local.local_ItemClass`) (`local.local_Amount`) 0 null)
      (set `local.local_ThrowAway` true)
      (break)))
  (if (`local.local_ThrowAway`)
    (return)
    (else
      (`|SpawnActorFromClass` "/Game/InventorySystem/Blueprints/ItemClasses/bp_PickupActor.bp_PickupActor_C" (`KismetMathLibrary.MakeTransform` (`SceneComponent.K2_GetComponentLocation` (`Character.CapsuleComponent` (`self.TopDownCharRef`))) (.rotation (`.WorldView_36_43EFD57C4C969519E567A989749D17E2` (break `/Game/InventorySystem/Blueprints/Structures/s_ItemInfo` (defaults `Object` (`local.local_ItemClass`))))) (.scale (`.WorldView_36_43EFD57C4C969519E567A989749D17E2` (break `/Game/InventorySystem/Blueprints/Structures/s_ItemInfo` (defaults `Object` (`local.local_ItemClass`)))))) "Undefined" "OverrideRootScale" null (`local.local_ItemClass`) (`local.local_Amount`) 0 null)
      (return))))

(fn `-SwapSlots`
  (params (Index1 :type Integer) (Index2 :type Integer))
  (returns (`Success?` :type Boolean))
  (locals (local_Index1 :type Integer) (local_Index2 :type Integer) (local_Slot2 :type "/Game/InventorySystem/Blueprints/Structures/s_InventorySlot Structure"))
  (bind _slots (`self.Slots`))
  (bind _returnvalue (`KismetArrayLibrary.Array_LastIndex` (`self.Slots`)))
  (set `local.local_Index1` Index1)
  (set `local.local_Index2` Index2)
  (if (or (> (`local.local_Index1`) _returnvalue) (> (`local.local_Index2`) _returnvalue))
    (return false)
    (else
      (set `local.local_Slot2` (`|GetArrayItem` (`self.Slots`) (`local.local_Index2`)))
      (`KismetArrayLibrary.Array_Set` _slots (`local.local_Index2`) (`|GetArrayItem` _slots (`local.local_Index1`)))
      (`KismetArrayLibrary.Array_Set` (`self.Slots`) (`local.local_Index1`) (`local.local_Slot2`))
      (`self.UpdateSlotAtIndex` (`local.local_Index1`))
      (`self.UpdateSlotAtIndex` (`local.local_Index2`))
      (return true))))

(fn `UserConstructionScript`)