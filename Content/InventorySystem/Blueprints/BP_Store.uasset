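; BP_Store is an interactable store chest that opens a storage inventory for the player and can belong to a merchant NPC.
; It can roll starting items from a merchant data table, replaced by slots saved under its ID in CItemsWorld.
; Interaction lazily spawns a Bp_Storage, shows it and freezes movement, guarded by a DoOnce.
; Closing restores movement, registers the chest in CItemsWorld and has any merchant generate offers from the slots.
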(event `self.ReceiveBeginPlay`
  (if (`self.GenerateStartingItems?`)
    (`self.-GenerateStartingItems`)))

(event `self.InteractionRange.OnComponentBeginOverlap`
  (params (OverlappedComponent :type "PrimitiveComponent Object Reference") (OtherActor :type "Actor Object Reference") (OtherComp :type "PrimitiveComponent Object Reference") (OtherBodyIndex :type Integer) (bFromSweep :type Boolean) (SweepResult :type "HitResult Structure (by ref)"))
  (bind _astop_down_character (cast `/Game/Core/Blueprints/TopDownCharacter` OtherActor))
  (`SceneComponent.SetVisibility` (`self.ChestText`) true false)
  (set `/Game/Core/Blueprints/TopDownCharacter.NearbyChest` self _astop_down_character))

(event `self.InteractionRange.OnComponentEndOverlap`
  (params (OverlappedComponent :type "PrimitiveComponent Object Reference") (OtherActor :type "Actor Object Reference") (OtherComp :type "PrimitiveComponent Object Reference") (OtherBodyIndex :type Integer))
  (bind _astop_down_character (cast `/Game/Core/Blueprints/TopDownCharacter` OtherActor))
  (`SceneComponent.SetVisibility` (`self.ChestText`) false false)
  (set `/Game/Core/Blueprints/TopDownCharacter.NearbyChest` null _astop_down_character))

(event `OnInteract`
  (params (TopDownChar :type "/Game/Core/Blueprints/TopDownCharacter Object Reference"))
  (bind _storageactor (`self.StorageActor`))
  (bind _topdownchar (`self.TopDownChar`))
  (bind _charactermovement (`Character.CharacterMovement` _topdownchar))
  (bind _inventoryref (`/Game/Core/Blueprints/TopDownCharacter.InventoryRef` _topdownchar))
  (`/Engine/EditorBlueprintResources/StandardMacros.DoOnce` false :!label _label
    (:`Completed`
      (set `self.TopDownChar` TopDownChar)
      (bind (_res _slots) (`/Game/InventorySystem/Blueprints/components/c_ItemsWorld.-getSlots` (`/Game/Core/Blueprints/TopDownCharacter.c_ItemsWorld` (`self.TopDownChar`)) (`self.ID`)))
      (if _res
        (set `self.StartingItems` _slots))
      (`/Engine/EditorBlueprintResources/StandardMacros.IsValid` (`self.StorageActor`)
        (:`Is Valid`
          _)
        (:`Is Not Valid`
          (bind _returnvalue (`|SpawnActorFromClass` "/Game/InventorySystem/Blueprints/bp_Storage.bp_Storage_C" (`KismetMathLibrary.MakeTransform` (0.0 0.0 0.0)) "Undefined" "OverrideRootScale" null (`self.AmountOfSlots`) (`self.TopDownChar`) (`self.SlotsPerRow`) self (`self.StartingItems`) null))
          (set `self.StorageActor` _returnvalue)))
      (`/Game/InventorySystem/Widgets/Storage/w_StorageWidget.-GenerateSlotWidget` (`/Game/InventorySystem/Blueprints/bp_Storage.StorageWidget` _storageactor) _storageactor)
      (`/Game/InventorySystem/Blueprints/bp_Storage.-ShowHideStorage` _storageactor true)
      (`/Game/InventorySystem/Blueprints/bp_Inventory.-HideInvetory` _inventoryref)
      (`/Game/InventorySystem/Blueprints/bp_Inventory.-ShowInvetory` _inventoryref)
      (`CharacterMovementComponent.DisableMovement` _charactermovement)
      (`MovementComponent.StopMovementImmediately` _charactermovement))))

(event `OnStorageClosed`
  (bind _topdownchar (`self.TopDownChar`))
  (bind _inventoryref (`/Game/Core/Blueprints/TopDownCharacter.InventoryRef` _topdownchar))
  (`/Game/InventorySystem/Blueprints/bp_Storage.-ShowHideStorage` (`self.StorageActor`) false)
  (bind _npc (`self.NPC`)
    (:`then`
      (bind _asmerchant (cast `/Game/InventorySystem/Blueprints/NPC/Merchant` _npc)
        (:`then`
          (`/Game/InventorySystem/Blueprints/NPC/Merchant.-GenerateOffer` _asmerchant (`/Game/InventorySystem/Blueprints/bp_Storage.Slots` (`self.StorageActor`))))
        (:`CastFailed`
          _))
      (`/Game/InventorySystem/Blueprints/NPC/bp_MasterNPC.OffInteract` _npc))
    (:`else`
      _))
  (`CharacterMovementComponent.SetMovementMode` (`Character.CharacterMovement` _topdownchar) "MOVE_Walking" 0)
  (`/Game/InventorySystem/Blueprints/components/c_ItemsWorld.-AddChest` (`/Game/Core/Blueprints/TopDownCharacter.c_ItemsWorld` (`self.TopDownChar`)) (`self.ID`) self)
  (if (`/Game/InventorySystem/Blueprints/bp_Inventory.isVisible?` _inventoryref)
    (`/Game/InventorySystem/Blueprints/bp_Inventory.-HideInvetory` _inventoryref)
    (`/Game/InventorySystem/Blueprints/bp_Inventory.-ShowInvetory` _inventoryref)
    (goto _label :!via `Reset`)
    (else
      (goto _label :!via `Reset`))))

(fn `-GenerateStartingItems`
  (bind _outrownames (`DataTableFunctionLibrary.GetDataTableRowNames` "/Game/InventorySystem/Blueprints/DataTables/Table_MerchantStarterItems.Table_MerchantStarterItems"))
  (for _array_element _outrownames
    (bind _returnvalue (`|GetDataTableRow` "/Game/InventorySystem/Blueprints/DataTables/Table_MerchantStarterItems.Table_MerchantStarterItems" _array_element)
      (:`then`
        (bind (_itemclass _minamount _maxamount _chance) (break `/Game/InventorySystem/Blueprints/Structures/s_MerchantContent` _returnvalue))
        (if (and (`KismetSystemLibrary.IsValidClass` _itemclass) (>= _chance (`KismetMathLibrary.RandomIntegerInRange` 1 100)) true)
          (`KismetArrayLibrary.Array_Add` (`self.StartingItems`) (make `/Game/InventorySystem/Blueprints/Structures/s_InventorySlot` _itemclass (`KismetMathLibrary.RandomIntegerInRange` _minamount _maxamount)))))))
  (return))

(fn `UserConstructionScript`)