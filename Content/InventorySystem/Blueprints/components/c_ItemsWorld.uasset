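; Character component that records the persistent state of world pickups and chests for the inventory system.
; Pickups are stored per map with location, amount and ID; add and remove maintain the list, and load respawns those on the character's current map.
; Chest slots are saved and retrieved by chest ID.
; A gold lookup checks whether an ID is in the save game's TakenGold list, loading the TDCSave slot if needed.
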(event `self.ReceiveBeginPlay`
  ;[1 1 1] Ссылка на владельца компонента
  (set `self.TopDownCharacter` (cast `/Game/Core/Blueprints/TopDownCharacter` (`self.GetOwner`) :!pure true)))

(fn `-AddChest`
  (params (ID :type Integer) (Chest :type "/Game/InventorySystem/Blueprints/BP_Store Object Reference"))
  (locals (local_ID_Chest :type Integer) (local_res :type Boolean) (local_index :type Integer))
  (bind _chestsworld (`self.ChestsWorld`))
  (bind _s_chestsworld (make `/Game/InventorySystem/Blueprints/Structures/ItemsMap/s_ChestsWorld` (`local.local_ID_Chest`) (`/Game/InventorySystem/Blueprints/bp_Storage.Slots` (`/Game/InventorySystem/Blueprints/BP_Store.StorageActor` Chest))))
  (set `local.local_ID_Chest` ID)
  (for (_array_element _array_index) (`self.ChestsWorld`)
    (if (== (`.ID_3_1887BAA9416E2BE85A0ED1AB32F9F057` (break `/Game/InventorySystem/Blueprints/Structures/ItemsMap/s_ChestsWorld` _array_element)) (`local.local_ID_Chest`))
      (set `local.local_res` true)
      (set `local.local_index` _array_index)
      (break)))
  (if (`local.local_res`)
    (`KismetArrayLibrary.Array_Set` _chestsworld (`local.local_index`) _s_chestsworld)
    (else
      (`KismetArrayLibrary.Array_Add` _chestsworld _s_chestsworld)))
  (return))

(fn `-addItem`
  (params (Map :type "/Game/InventorySystem/Blueprints/Enums/e_maps Enum" :default "NewEnumerator0") (PickupActor :type "/Game/InventorySystem/Blueprints/ItemClasses/Classes/bp_MasterItem Class Reference") (Location :type "Transform Structure") (Amount :type Integer) (ID :type Integer))
  (locals (local_itemsInfo :type "Array of /Game/InventorySystem/Blueprints/Structures/ItemsMap/s_ItemsInfo Structure") (local_index :type Integer) (local_res :type Boolean))
  (bind _s_itemsinfo (make `/Game/InventorySystem/Blueprints/Structures/ItemsMap/s_ItemsInfo` PickupActor Location Amount ID))
  (bind _itemsonmaps (`self.ItemsOnMaps`))
  (for (_array_element _array_index) (`self.ItemsOnMaps`)
    (bind (_map _itemsinfo) (break `/Game/InventorySystem/Blueprints/Structures/ItemsMap/s_ItemsMap` _array_element))
    (if (`|EnumEquality` Map _map)
      (bind _output_get (set `local.local_itemsInfo` _itemsinfo))
      (`KismetArrayLibrary.Array_Add` _output_get _s_itemsinfo)
      (set `local.local_index` _array_index)
      (set `local.local_res` true)
      (break)))
  (if (`local.local_res`)
    (`KismetArrayLibrary.Array_Set` _itemsonmaps (`local.local_index`) (make `/Game/InventorySystem/Blueprints/Structures/ItemsMap/s_ItemsMap` Map (`local.local_itemsInfo`)))
    (else
      (`KismetArrayLibrary.Array_Add` _itemsonmaps (make `/Game/InventorySystem/Blueprints/Structures/ItemsMap/s_ItemsMap` Map (`|MakeArray` _s_itemsinfo)))))
  (`/Engine/EditorBlueprintResources/StandardMacros.IncrementInt` (`self.LastItemsID`)
    (:`  `
      (return))))

(fn `-getIdGold`
  (params (ID :type Integer))
  (returns (local_res1 :type Boolean))
  (locals (local_Id :type Integer) (local_res :type Boolean))
  (bind _astop_down_character (cast `/Game/Core/Blueprints/TopDownCharacter` (`GameplayStatics.GetPlayerCharacter` 0) :!pure true))
  (set `local.local_Id` ID)
  (`/Engine/EditorBlueprintResources/StandardMacros.IsValid` (`/Game/Core/Blueprints/TopDownCharacter.SaveGameObject` _astop_down_character)
    (:`Is Valid`
      _)
    (:`Is Not Valid`
      (bind _returnvalue (`GameplayStatics.LoadGameFromSlot` "TDCSave"))
      (bind _astdcsave (cast `/Game/InventorySystem/Blueprints/SaveGames/TDCSave` _returnvalue))
      (bind _output_get (set `/Game/Core/Blueprints/TopDownCharacter.SaveGameObject` _astdcsave _astop_down_character))))
  (set `self.TakenGold` (`/Game/InventorySystem/Blueprints/SaveGames/TDCSave.TakenGold` _output_get))
  (for _array_element (`self.TakenGold`)
    (if (== _array_element (`local.local_Id`))
      (set `local.local_res` true)
      (break)))
  (return (`local.local_res`)))

(fn `-getSlots`
  (params (ID :type Integer))
  (returns (res :type Boolean) (Slots :type "Array of /Game/InventorySystem/Blueprints/Structures/s_InventorySlot Structure"))
  (locals (local_ID :type Integer) (local_res :type Boolean) (local_index :type Integer))
  (set `local.local_ID` ID)
  (for (_array_element _array_index) (`self.ChestsWorld`)
    (if (== (`.ID_3_1887BAA9416E2BE85A0ED1AB32F9F057` (break `/Game/InventorySystem/Blueprints/Structures/ItemsMap/s_ChestsWorld` _array_element)) (`local.local_ID`))
      (set `local.local_res` true)
      (set `local.local_index` _array_index)
      (break)))
  (if (`local.local_res`)
    (return true (`.Slot_6_43B3B19A41C5504F71A2B5A3299D845B` (break `/Game/InventorySystem/Blueprints/Structures/ItemsMap/s_ChestsWorld` (`|GetArrayItem` (`self.ChestsWorld`) (`local.local_index`)))))
    (else
      (return false))))

(fn `-loadGame`
  (params (itemsLoad :type "/Game/InventorySystem/Blueprints/Structures/ItemsMap/s_ItemsOnMaps_LoadSaveGame Structure"))
  (locals (local_itemsOnMap :type "Array of /Game/InventorySystem/Blueprints/Structures/ItemsMap/s_ItemsInfo Structure"))
  (bind (_lastitemsid _items) (break `/Game/InventorySystem/Blueprints/Structures/ItemsMap/s_ItemsOnMaps_LoadSaveGame` itemsLoad))
  (set `self.LastItemsID` _lastitemsid)
  (bind _output_get (set `self.ItemsOnMaps` _items))
  (for _array_element _output_get
    (bind (_map _itemsinfo) (break `/Game/InventorySystem/Blueprints/Structures/ItemsMap/s_ItemsMap` _array_element))
    (if (`|EnumEquality` _map (`/Game/Core/Blueprints/TopDownCharacter.Map` (`self.TopDownCharacter`)))
      (set `local.local_itemsOnMap` _itemsinfo)
      (break)))
  (for _array_element_2 (`local.local_itemsOnMap`)
    (bind (_pickupactor _location _amount _id) (break `/Game/InventorySystem/Blueprints/Structures/ItemsMap/s_ItemsInfo` _array_element_2))
    (`|SpawnActorFromClass` "/Game/InventorySystem/Blueprints/ItemClasses/bp_PickupActor.bp_PickupActor_C" _location "AlwaysSpawn" "OverrideRootScale" null _pickupactor _amount _id null))
  (return))

(fn `-removeItem`
  (params (Map :type "/Game/InventorySystem/Blueprints/Enums/e_maps Enum" :default "NewEnumerator0") (Id :type Integer))
  (locals (local_arr1_index :type Integer) (local_arr1_res :type Boolean) (local_itemsInfo :type "Array of /Game/InventorySystem/Blueprints/Structures/ItemsMap/s_ItemsInfo Structure") (local_Id :type Integer) (local_map :type "/Game/InventorySystem/Blueprints/Enums/e_maps Enum" :default "NewEnumerator0"))
  (bind _itemsonmaps (`self.ItemsOnMaps`))
  (bind _local_arr1_index (`local.local_arr1_index`))
  (set `local.local_map` Map)
  (set `local.local_Id` Id)
  (for (_array_element _array_index) (`self.ItemsOnMaps`)
    (bind (_map _itemsinfo) (break `/Game/InventorySystem/Blueprints/Structures/ItemsMap/s_ItemsMap` _array_element))
    (if (`|EnumEquality` _map (`local.local_map`))
      (set `local.local_arr1_index` _array_index)
      (set `local.local_arr1_res` true)
      (break)))
  (if (`local.local_arr1_res`)
    (set `local.local_itemsInfo` _itemsinfo)
    (for (_array_element_2 _array_index_2) (`local.local_itemsInfo`)
      (if (== (`.ID_11_A7A224E047DDDC20E2B1F396957E142A` (break `/Game/InventorySystem/Blueprints/Structures/ItemsMap/s_ItemsInfo` _array_element_2)) (`local.local_Id`))
        (`KismetArrayLibrary.Array_Remove` (`local.local_itemsInfo`) _array_index_2)))
    (if (not (> (`KismetArrayLibrary.Array_Length` (`local.local_itemsInfo`)) 0))
      (`KismetArrayLibrary.Array_Remove` _itemsonmaps _local_arr1_index)
      (else
        (`KismetArrayLibrary.Array_Set` _itemsonmaps _local_arr1_index (make `/Game/InventorySystem/Blueprints/Structures/ItemsMap/s_ItemsMap` (`local.local_map`) (`local.local_itemsInfo`)))))
    (return)
    (else
      (return))))