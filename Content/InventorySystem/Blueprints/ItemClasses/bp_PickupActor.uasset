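; World pickup for inventory items and gold, taking its mesh, scale and interaction radius from the ItemClass defaults and spinning on Tick.
; Overlap joins the character's nearby-pickup queue, showing the first's label, or collects immediately with HasPickupCommand.
; OnPickUp records IDs, keeping any inventory leftover in the world; gold goes to the character's balance and self-destroys on BeginPlay if already taken.
; Cursor hover swaps material and cursor and shows the label.
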(event `self.ReceiveBeginPlay`
  ;[1 1 1] BeginPlay
  (`self.-UpdateText`)
  (`self.-TakenGold`))

(event `self.ReceiveTick`
  (params (DeltaSeconds :type "Float (single-precision)"))
  (bind _skeletalmesh (`self.SkeletalMesh`))
  (bind _rotation (`self.Rotation`))
  ;[1 1 1] Tick
  ;;[1 1 1] Rotation Item
  (`KismetSystemLibrary.Delay` 0.001)
  (bind _staticmesh (`self.StaticMesh`)
    (:`then`
      (`SceneComponent.K2_SetWorldRotation` _staticmesh (`KismetMathLibrary.MakeRotator` (.roll (`SceneComponent.K2_GetComponentRotation` _staticmesh)) (.pitch (`SceneComponent.K2_GetComponentRotation` _staticmesh)) (`self.Rotation`)) false false))
    (:`else`
      (`SceneComponent.K2_SetWorldRotation` _skeletalmesh (`KismetMathLibrary.MakeRotator` (.roll (`SceneComponent.K2_GetComponentRotation` _skeletalmesh)) (.pitch (`SceneComponent.K2_GetComponentRotation` _skeletalmesh)) (`self.Rotation`)) false false)))
  (set `self.Rotation` (+ _rotation 0.1))
  (if (> _rotation 360.0)
    (set `self.Rotation` 0.0)))

(event `OnPickUp`
  (params (TopDownChar :type "/Game/Core/Blueprints/TopDownCharacter Object Reference"))
  (bind _inventoryref (`/Game/Core/Blueprints/TopDownCharacter.InventoryRef` (`self.TopDownChar`)))
  (bind _nearbypickupactors (`/Game/Core/Blueprints/TopDownCharacter.NearbyPickupActors` (`self.TopDownChar`)))
  (bind _inventoryref_2 (`/Game/Core/Blueprints/TopDownCharacter.InventoryRef` (`self.TopDownChar`)))
  (bind _output (`|GetArrayItem` _nearbypickupactors))
  (bind _lootedpickups (`/Game/InventorySystem/Blueprints/bp_Inventory.LootedPickups` (`/Game/Core/Blueprints/TopDownCharacter.InventoryRef` (`self.TopDownChar`))))
  (set `self.TopDownChar` TopDownChar)
  (if (!= (`self.ItemClass`) "/Game/InventorySystem/Blueprints/ItemClasses/Classes/bp_ItemGold.bp_ItemGold_C")
    (`/Engine/EditorBlueprintResources/StandardMacros.IsValid` _inventoryref
      (:`Is Valid`
        (bind (_success2_ _rest2) (`/Game/InventorySystem/Blueprints/bp_Inventory.-AddItem` _inventoryref (`self.ItemClass`) (`self.Amount`) true (`self.ID`)))
        (if _success2_
          (if (> _rest2 0)
            (set `self.Amount` _rest2)
            (`self.-UpdateText`)
            (`KismetArrayLibrary.Array_Add` _lootedpickups (make `/Game/InventorySystem/Blueprints/Structures/s_SavedPickup` (`self.ID`) (`self.Amount`)))
            (else
              (`KismetArrayLibrary.Array_Add` _lootedpickups (make `/Game/InventorySystem/Blueprints/Structures/s_SavedPickup` (`self.ID`)))
              (`KismetArrayLibrary.Array_RemoveItem` _nearbypickupactors self)
              (`/Engine/EditorBlueprintResources/StandardMacros.IsValid` _output
                (:`Is Valid`
                  (`SceneComponent.SetVisibility` (`/Game/InventorySystem/Blueprints/ItemClasses/bp_PickupActor.PickupText` _output) true false))
                (:`Is Not Valid`
                  _))
              (if (`self.Hovered?`)
                (set `PlayerController.CurrentMouseCursor` "Default" (`GameplayStatics.GetPlayerController` 0))
                (`self.K2_DestroyActor`)
                (else
                  (`self.K2_DestroyActor`))))))))
    (else
      ;[1 1 1] Gold
      (`KismetArrayLibrary.Array_AddUnique` (`/Game/InventorySystem/Blueprints/components/c_ItemsWorld.TakenGold` (`/Game/Core/Blueprints/TopDownCharacter.c_ItemsWorld` (`self.TopDownChar`))) (`self.ID`))
      (`/Game/Core/Blueprints/TopDownCharacter.-IncreaseGold` (`self.TopDownChar`) (`self.Amount`))
      (set `/Game/InventorySystem/Blueprints/bp_Inventory.ShowObtainedMessage?` true _inventoryref_2)
      (`/Game/InventorySystem/Blueprints/bp_Inventory.-ShowObtainedItem` _inventoryref_2 (`self.ItemClass`) (`self.Amount`))
      (`self.K2_DestroyActor`))))

(event `self.Sphere.OnComponentBeginOverlap`
  (params (OverlappedComponent :type "PrimitiveComponent Object Reference") (OtherActor :type "Actor Object Reference") (OtherComp :type "PrimitiveComponent Object Reference") (OtherBodyIndex :type Integer) (bFromSweep :type Boolean) (SweepResult :type "HitResult Structure (by ref)"))
  (bind _astop_down_character (cast `/Game/Core/Blueprints/TopDownCharacter` OtherActor))
  (`PrimitiveComponent.SetCollisionEnabled` (`self.StaticMesh`) "NoCollision")
  (if (`self.hasPickupCommand?`)
    (`self.OnPickUp` _astop_down_character)
    (else
      (bind _nearbypickupactors (`/Game/Core/Blueprints/TopDownCharacter.NearbyPickupActors` _astop_down_character))
      (if (> (`KismetArrayLibrary.Array_Length` _nearbypickupactors) 0)
        (`KismetArrayLibrary.Array_Add` _nearbypickupactors self)
        (else
          (`SceneComponent.SetVisibility` (`self.PickupText`) true false)
          (`KismetArrayLibrary.Array_Add` _nearbypickupactors self)
          (set `self.isInRange?` true))))))

(event `self.Sphere.OnComponentEndOverlap`
  (params (OverlappedComponent :type "PrimitiveComponent Object Reference") (OtherActor :type "Actor Object Reference") (OtherComp :type "PrimitiveComponent Object Reference") (OtherBodyIndex :type Integer))
  (bind _astop_down_character (cast `/Game/Core/Blueprints/TopDownCharacter` OtherActor))
  (`PrimitiveComponent.SetCollisionEnabled` (`self.StaticMesh`) "QueryAndPhysics")
  (set `self.isInRange?` false)
  (bind _nearbypickupactors (`/Game/Core/Blueprints/TopDownCharacter.NearbyPickupActors` _astop_down_character))
  (bind _output (`|GetArrayItem` _nearbypickupactors))
  (if (and (`KismetSystemLibrary.IsValid` _output) (== _output self))
    (`SceneComponent.SetVisibility` (`self.PickupText`) false false)
    (`KismetArrayLibrary.Array_RemoveItem` _nearbypickupactors self)
    (bind _output_2 (`|GetArrayItem` _nearbypickupactors))
    (`/Engine/EditorBlueprintResources/StandardMacros.IsValid` _output_2
      (:`Is Valid`
        (`SceneComponent.SetVisibility` (`/Game/InventorySystem/Blueprints/ItemClasses/bp_PickupActor.PickupText` _output_2) true false)))
    (else
      (`KismetArrayLibrary.Array_RemoveItem` _nearbypickupactors self))))

(event `self.StaticMesh.OnBeginCursorOver`
  (params (TouchedComponent :type "PrimitiveComponent Object Reference"))
  (`self.-OnHovered` :!label _label))

(event `self.CursorSphere.OnBeginCursorOver`
  (params (TouchedComponent :type "PrimitiveComponent Object Reference"))
  (goto _label))

(event `self.CursorSphere.OnEndCursorOver`
  (params (TouchedComponent :type "PrimitiveComponent Object Reference"))
  (`self.-OnUnhovered` :!label _label_2))

(event `self.StaticMesh.OnEndCursorOver`
  (params (TouchedComponent :type "PrimitiveComponent Object Reference"))
  (goto _label_2))

(fn `-OnHovered`
  (set `self.Hovered?` true)
  (set `PlayerController.CurrentMouseCursor` "Hand" (`GameplayStatics.GetPlayerController` 0))
  (bind _staticmesh (`self.StaticMesh`)
    (:`then`
      (`PrimitiveComponent.SetMaterial` _staticmesh 0 "/Game/InventorySystem/Materials/HoveredPickupMat.HoveredPickupMat"))
    (:`else`
      _))
  (`SceneComponent.SetVisibility` (`self.PickupText`) true false)
  (return))

(fn `-OnUnhovered`
  (set `self.Hovered?` false)
  (set `PlayerController.CurrentMouseCursor` "Default" (`GameplayStatics.GetPlayerController` 0))
  (bind _staticmesh (`self.StaticMesh`)
    (:`then`
      (`PrimitiveComponent.SetMaterial` _staticmesh 0 (`self.OriginalMaterial`)))
    (:`else`
      _))
  (`SceneComponent.SetVisibility` (`self.PickupText`) (`self.isInRange?`) false)
  (return))

(fn `-TakenGold`
  (if (== (`self.ItemClass`) "/Game/InventorySystem/Blueprints/ItemClasses/Classes/bp_ItemGold.bp_ItemGold_C")
    (bind _local_res1 (`/Game/InventorySystem/Blueprints/components/c_ItemsWorld.-getIdGold` (`/Game/Core/Blueprints/TopDownCharacter.c_ItemsWorld` (cast `/Game/Core/Blueprints/TopDownCharacter` (`GameplayStatics.GetPlayerCharacter` 0) :!pure true)) (`self.ID`)))
    (if _local_res1
      (`self.K2_DestroyActor`))))

(fn `-UpdateText`
  (bind _asw_pickup_text (cast `/Game/InventorySystem/Widgets/w_PickupText` (`WidgetComponent.GetUserWidgetObject` (`self.PickupText`)))
    (:`then`
      (`TextBlock.SetText` (`/Game/InventorySystem/Widgets/w_PickupText.NameText` _asw_pickup_text) (`|FormatText` "{Name} ({Amount})" (`.Name_2_AC4B5FB64D104CB9950EDEB297EA0383` (break `/Game/InventorySystem/Blueprints/Structures/s_ItemInfo` (defaults `Object` (`self.ItemClass`)))) (`KismetTextLibrary.Conv_IntToText` (`self.Amount`)))))
    (:`CastFailed`
      _))
  (return))

(fn `UserConstructionScript`
  (bind _itemclass (`self.ItemClass`))
  (bind _staticmesh (`self.StaticMesh`))
  (bind (_name _description _icon _canbeused_ _usetext _canbestacked_ _category _pickupmesh _meshscale _interactradius) (break `/Game/InventorySystem/Blueprints/Structures/s_ItemInfo` (defaults `Object` _itemclass)))
  (`|ExecutionSequence`
    (:`then_0`
      (if (`KismetSystemLibrary.IsValidClass` _itemclass)
        (`StaticMeshComponent.SetStaticMesh` _staticmesh _pickupmesh)
        (set `self.OriginalMaterial` (`PrimitiveComponent.GetMaterial` _staticmesh 0))
        (`SceneComponent.SetRelativeScale3D` _staticmesh _meshscale)
        (`SphereComponent.SetSphereRadius` (`self.Sphere`) _interactradius false)))
    (:`then_1`
      ;[1 1 1] Радиус сферы для выделения курсором
      (`SphereComponent.SetSphereRadius` (`self.CursorSphere`) (/ (`SphereComponent.SphereRadius` (`self.Sphere`)) 4.0) true))))