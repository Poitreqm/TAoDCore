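; Merchant NPC that the player can either trade with or rob.
; Hovering outlines it and sets the cursor, with Left Ctrl selecting robbery; a proximity sphere registers it as the nearby NPC and shows its label.
; Interacting opens a centered shop widget and halts player movement, or opens the linked chest when robbing, each guarded by a DoOnce reset on shop close or interaction end.
; GenerateOffer fills the offer list from valid starting item classes.
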(event `self.ReceiveBeginPlay`
  (`parent.ReceiveBeginPlay`))

(event `self.OnShopClosed`
  (bind _shopwidget (`self.ShopWidget`))
  (bind _topdownchar (`self.TopDownChar`))
  (bind _inventoryref (`/Game/Core/Blueprints/TopDownCharacter.InventoryRef` _topdownchar))
  (bind _charactermovement (`Character.CharacterMovement` _topdownchar))
  (`parent.OnShopClosed`)
  (`Widget.RemoveFromParent` (`self.ShopWidget`))
  (set `self.ShopWidget` null)
  (goto _label :!via `Reset`))

(event `self.OnInteract`
  (params (TopDownCharacter :type "/Game/Core/Blueprints/TopDownCharacter Object Reference"))
  (bind _shopwidget (`self.ShopWidget`))
  (bind _topdownchar (`self.TopDownChar`))
  (bind _inventoryref (`/Game/Core/Blueprints/TopDownCharacter.InventoryRef` _topdownchar))
  (bind _charactermovement (`Character.CharacterMovement` _topdownchar))
  (`parent.OnInteract` TopDownCharacter)
  (set `self.TopDownChar` TopDownCharacter)
  (if (not (`self.PlayerGrab?`))
    ;[1 1 1] Совершаем покупку у продавца
    (`/Engine/EditorBlueprintResources/StandardMacros.DoOnce` false :!label _label
      (:`Completed`
        (bind _returnvalue (`|CreateWidget` "/Game/InventorySystem/Widgets/w_ShopWidget.w_ShopWidget_C" null self (`self.TopDownChar`)))
        (set `self.ShopWidget` _returnvalue)
        (`UserWidget.SetPositionInViewport` _shopwidget (0.0 0.0) false)
        (`UserWidget.SetAnchorsInViewport` _shopwidget (make `Anchors` (0.5 0.5) (0.5 0.5)))
        (`UserWidget.SetAlignmentInViewport` _shopwidget (0.5 0.5))
        (`UserWidget.AddToViewport` _shopwidget 5)
        (`/Game/InventorySystem/Blueprints/bp_Inventory.-HideInvetory` _inventoryref)
        (`/Game/InventorySystem/Blueprints/bp_Inventory.-ShowInvetory` _inventoryref)
        (set `/Game/Core/Blueprints/TopDownCharacter.IsShopOpen?` true _topdownchar)
        (`CharacterMovementComponent.DisableMovement` _charactermovement)
        (`MovementComponent.StopMovementImmediately` _charactermovement)))
    (else
      ;[1 1 1] Грабим
      (`/Engine/EditorBlueprintResources/StandardMacros.DoOnce` false :!label _label_2
        (:`Completed`
          (`self.bpChest`
            (:`then`
              (`/Game/InventorySystem/Blueprints/BP_Store.OnInteract` (`self.bpChest`) (`self.TopDownChar`)))
            (:`else`)))))))

(event `self.OffInteract`
  ;[1 1 1] Грабим
  (`parent.OffInteract`)
  (goto _label_2 :!via `Reset`))

(event `self.CapsuleComponent.OnBeginCursorOver`
  (params (TouchedComponent :type "PrimitiveComponent Object Reference"))
  (bind _astop_down_character (cast `/Game/Core/Blueprints/TopDownCharacter` (`Controller.K2_GetPawn` (`GameplayStatics.GetPlayerController` 0))))
  (set `/Game/Core/Blueprints/TopDownCharacter.MerchantCursor` self _astop_down_character)
  (`self.-Set_Cursor` _astop_down_character)
  (`PrimitiveComponent.SetRenderCustomDepth` (`self.Mesh`) true))

(event `self.CapsuleComponent.OnEndCursorOver`
  (params (TouchedComponent :type "PrimitiveComponent Object Reference"))
  (set `PlayerController.CurrentMouseCursor` "Default" (`GameplayStatics.GetPlayerController` 0))
  (bind _astop_down_character (cast `/Game/Core/Blueprints/TopDownCharacter` (`Controller.K2_GetPawn` (`GameplayStatics.GetPlayerController` 0))))
  (set `/Game/Core/Blueprints/TopDownCharacter.MerchantCursor` null _astop_down_character)
  (if (not (`self.isSelected?`))
    (`PrimitiveComponent.SetRenderCustomDepth` (`self.Mesh`) false)))

(event `self.Sphere_0.OnComponentBeginOverlap`
  (params (OverlappedComponent :type "PrimitiveComponent Object Reference") (OtherActor :type "Actor Object Reference") (OtherComp :type "PrimitiveComponent Object Reference") (OtherBodyIndex :type Integer) (bFromSweep :type Boolean) (SweepResult :type "HitResult Structure (by ref)"))
  (bind _astop_down_character (cast `/Game/Core/Blueprints/TopDownCharacter` OtherActor))
  (set `/Game/Core/Blueprints/TopDownCharacter.NearbyNPC` self _astop_down_character)
  (`SceneComponent.SetVisibility` (`self.MerchantText`) true false))

(event `self.Sphere_0.OnComponentEndOverlap`
  (params (OverlappedComponent :type "PrimitiveComponent Object Reference") (OtherActor :type "Actor Object Reference") (OtherComp :type "PrimitiveComponent Object Reference") (OtherBodyIndex :type Integer))
  (bind _astop_down_character (cast `/Game/Core/Blueprints/TopDownCharacter` OtherActor))
  (set `/Game/Core/Blueprints/TopDownCharacter.NearbyNPC` null _astop_down_character)
  (`SceneComponent.SetVisibility` (`self.MerchantText`) false false))

(fn `-GenerateOffer`
  (params (StartingItems :type "Array of /Game/InventorySystem/Blueprints/Structures/s_InventorySlot Structure"))
  (bind _offer (`self.Offer`))
  (`KismetArrayLibrary.Array_Clear` _offer)
  (for _array_element StartingItems
    (bind _itemclass (break `/Game/InventorySystem/Blueprints/Structures/s_InventorySlot` _array_element))
    (if (`KismetSystemLibrary.IsValidClass` _itemclass)
      (`KismetArrayLibrary.Array_Add` _offer _itemclass)))
  (return))

(fn `-Set_Cursor`
  (params (Player :type "/Game/Core/Blueprints/TopDownCharacter Object Reference"))
  (if (`/Game/Core/Blueprints/TopDownCharacter.LeftCtrl` Player)
    (set `self.PlayerGrab?` true)
    (set `PlayerController.CurrentMouseCursor` "GrabHandClosed" (`GameplayStatics.GetPlayerController` 0))
    (else
      (set `self.PlayerGrab?` false)
      (set `PlayerController.CurrentMouseCursor` "TextEditBeam" (`GameplayStatics.GetPlayerController` 0)))))

(fn `UserConstructionScript`)