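; Enemy NPC for a top-down game that can be killed and then robbed through a linked chest.
; Player overlap with its Interact component marks it dead, ragdolls the mesh and sets the capsule to query-only collision.
; Once dead, OnInteract forwards to BpChest through a DoOnce that OffInteract resets.
; Hover events switch cursor and text between attack and rob, outlining the corpse via custom depth and the player's post-process volume.
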(event `self.OnInteract`
  (params (TopDownCharacter :type "/Game/Core/Blueprints/TopDownCharacter Object Reference"))
  (`parent.OnInteract` TopDownCharacter)
  (set `self.TopDownChar` TopDownCharacter)
  (if (`self.isDeath?`)
    (`/Engine/EditorBlueprintResources/StandardMacros.DoOnce` false :!label _label
      (:`Completed`
        (`self.bpChest`
          (:`then`
            (`/Game/InventorySystem/Blueprints/BP_Store.OnInteract` (`self.bpChest`) (`self.TopDownChar`)))
          (:`else`))))))

(event `self.OffInteract`
  (`parent.OffInteract`)
  (goto _label :!via `Reset`))

(event `self.CapsuleComponent.OnBeginCursorOver`
  (params (TouchedComponent :type "PrimitiveComponent Object Reference"))
  (if (not (`self.isDeath?`))
    (set `PlayerController.CurrentMouseCursor` "ResizeLeftRight" (`GameplayStatics.GetPlayerController` 0))
    (`/Game/Core/Blueprints/TopDownCharacter.-SetCursorText` (cast `/Game/Core/Blueprints/TopDownCharacter` (`GameplayStatics.GetPlayerCharacter` 0) :!pure true) "Attack")))

(event `self.CapsuleComponent.OnEndCursorOver`
  (params (TouchedComponent :type "PrimitiveComponent Object Reference"))
  (if (not (`self.isDeath?`))
    (set `PlayerController.CurrentMouseCursor` "Default" (`GameplayStatics.GetPlayerController` 0))
    (`/Game/Core/Blueprints/TopDownCharacter.-SetCursorText` (cast `/Game/Core/Blueprints/TopDownCharacter` (`GameplayStatics.GetPlayerCharacter` 0) :!pure true) "")))

(event `self.Interact.OnComponentBeginOverlap`
  (params (OverlappedComponent :type "PrimitiveComponent Object Reference") (OtherActor :type "Actor Object Reference") (OtherComp :type "PrimitiveComponent Object Reference") (OtherBodyIndex :type Integer) (bFromSweep :type Boolean) (SweepResult :type "HitResult Structure (by ref)"))
  (cast `/Game/Core/Blueprints/TopDownCharacter` OtherActor)
  (`PrimitiveComponent.SetSimulatePhysics` (`self.Mesh`) true)
  (`PrimitiveComponent.SetCollisionEnabled` (`self.CapsuleComponent`) "QueryOnly")
  (set `self.isDeath?` true))

(event `self.Mesh.OnBeginCursorOver`
  (params (TouchedComponent :type "PrimitiveComponent Object Reference"))
  (if (`self.isDeath?`)
    (set `PlayerController.CurrentMouseCursor` "GrabHandClosed" (`GameplayStatics.GetPlayerController` 0))
    (set `PostProcessVolume.bEnabled` true (`/Game/Core/Blueprints/TopDownCharacter.PostProcessVolumeEnemy` (cast `/Game/Core/Blueprints/TopDownCharacter` (`GameplayStatics.GetPlayerCharacter` 0) :!pure true)))
    (`PrimitiveComponent.SetRenderCustomDepth` (`self.Mesh`) true)
    (`/Game/Core/Blueprints/TopDownCharacter.-SetCursorText` (cast `/Game/Core/Blueprints/TopDownCharacter` (`GameplayStatics.GetPlayerCharacter` 0) :!pure true) "to rob")))

(event `self.Mesh.OnEndCursorOver`
  (params (TouchedComponent :type "PrimitiveComponent Object Reference"))
  (set `PlayerController.CurrentMouseCursor` "Default" (`GameplayStatics.GetPlayerController` 0))
  (set `PostProcessVolume.bEnabled` false (`/Game/Core/Blueprints/TopDownCharacter.PostProcessVolumeEnemy` (cast `/Game/Core/Blueprints/TopDownCharacter` (`GameplayStatics.GetPlayerCharacter` 0) :!pure true)))
  (`PrimitiveComponent.SetRenderCustomDepth` (`self.Mesh`) false)
  (`/Game/Core/Blueprints/TopDownCharacter.-SetCursorText` (cast `/Game/Core/Blueprints/TopDownCharacter` (`GameplayStatics.GetPlayerCharacter` 0) :!pure true) ""))

(fn `UserConstructionScript`
  (`parent.UserConstructionScript`))